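; Player character that rebuilds its customized look on BeginPlay from the CharCustomization save slot.
; Selected meshes either replace the main Mesh or become added components slaved to it through Master Pose; all morph values are set on the main Mesh.
; Selected attachments spawn as skeletal or static components on sockets, with dynamic material instances coloring parts and attachments.
; Turn and look input are wired, while movement axis events are unconnected.
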(event EventBeginPlay
  ;[1 1 1] Update Character On Begin Play
  (CallFunction|UpdateCustomizedCharacter))

(event Input|AxisEvents|InputAxisTurn
  (params (AxisValue :type Float%20%28single-precision%29))
  ;[1 1 1] Character Inputs
  (Pawn|Input|AddControllerYawInput AxisValue))

(event Input|AxisEvents|InputAxisLookUp
  (params (AxisValue :type Float%20%28single-precision%29))
  ;[1 1 1] Character Inputs
  (Pawn|Input|AddControllerPitchInput AxisValue))

(event Input|AxisEvents|InputAxisMoveForward
  (params (AxisValue :type Float%20%28single-precision%29))
  ;[1 1 1] Character Inputs
)

(event Input|AxisEvents|InputAxisMoveRight
  (params (AxisValue :type Float%20%28single-precision%29))
  ;[1 1 1] Character Inputs
)

(fn ConstructionScript)

(fn UpdateCustomizedCharacter
  ;[1 1 1] Get Saved Customization Info
  (bind _returnvalue (SaveGame|LoadGamefromSlot "CharCustomization"))
  (bind _asbp_dccsave_game (Utilities|Casting|CastToBP_DCCSaveGame _returnvalue))
  (for _array_element (Variables|/Game/DynamicCC/Blueprints/Data/SaveGame/BP_DCCSaveGame.BP_DCCSaveGame_C|GetCustomizationMaster _asbp_dccsave_game)
    (LocalVariables|SetLocAvailableMeshes (.AvailableMeshes (Utilities|Struct|BreakStruct_SavedCustomization _array_element)))
    (LocalVariables|SetLocAvailableAttachments (.AvailableAttachments (Utilities|Struct|BreakStruct_SavedCustomization _array_element)))
    ;[1 1 1] Update/Add Skeletal Mesh Components
    (for _array_element_2 (LocalVariables|GetLocAvailableMeshes)
      (if (.IsSelected (Utilities|Struct|BreakStruct_SavedMeshes _array_element_2))
        (if (Utilities|Struct|BreakStruct_MasterPoseSetup (.MasterPoseSetup (Utilities|Struct|BreakStruct_SavedMeshes _array_element_2)))
          (Class|SkinnedMeshComponent|SetSkeletalMesh (Variables|Character|GetMesh) (.SkeletalMesh (Utilities|Struct|BreakStruct_SavedMeshes _array_element_2)) true)
          (for _array_element_3 (.MorphTargets (Utilities|Struct|BreakStruct_SavedMeshes _array_element_2))
            (Components|SkeletalMesh|SetMorphTarget (Variables|Character|GetMesh) (.MorphTargetName (Utilities|Struct|BreakStruct_MorphTargetSetup _array_element_3)) (Math|Float|MapRangeClamped (.DefaultValue (Utilities|Struct|BreakStruct_MorphTargetSetup _array_element_3)) (.x (.NormalizeToRange (Utilities|Struct|BreakStruct_MorphTargetSetup _array_element_3))) (.y (.NormalizeToRange (Utilities|Struct|BreakStruct_MorphTargetSetup _array_element_3))) -1.0 1.0) true))
          (for _array_element_4 (.ColorSchemes (Utilities|Struct|BreakStruct_SavedMeshes _array_element_2))
            (for _array_element_5 (.TargetMaterials (Utilities|Struct|BreakStruct_SavedColorSchemes _array_element_4))
              (bind _returnvalue_2 (Rendering|Material|CreateDynamicMaterialInstance (Variables|Character|GetMesh) (.SlotIndex (Utilities|Struct|BreakStruct_MaterialSetup _array_element_5)) (.MaterialReference (Utilities|Struct|BreakStruct_MaterialSetup _array_element_5)) "None" :!class /Script/Engine.PrimitiveComponent))
              (for _array_element_6 (.Colors (Utilities|Struct|BreakStruct_SavedColorSchemes _array_element_4))
                (if (.IsSelected (Utilities|Struct|BreakStruct_SavedColorSelection _array_element_6))
                  (Rendering|Material|SetVectorParameterValue _returnvalue_2 (.ParamaterName (Utilities|Struct|BreakStruct_MaterialSetup _array_element_5)) (.Color (Utilities|Struct|BreakStruct_SavedColorSelection _array_element_6)) :!class /Script/Engine.MaterialInstanceDynamic)))))
          (else
            (bind _returnvalue_3 (AddComponent|AddSkeletalMeshComponent false))
            (Class|SkinnedMeshComponent|SetSkeletalMesh _returnvalue_3 (.SkeletalMesh (Utilities|Struct|BreakStruct_SavedMeshes _array_element_2)) true)
            (Utilities|Array|Add (LocalVariables|GetSKMeshes) _returnvalue_3)
            (Transformation|AttachComponentToComponent _returnvalue_3 (Variables|Character|GetMesh) "None" "SnapToTarget" "SnapToTarget" "KeepWorld" true)
            (for _array_element_7 (.MorphTargets (Utilities|Struct|BreakStruct_SavedMeshes _array_element_2))
              (Components|SkeletalMesh|SetMorphTarget (Variables|Character|GetMesh) (.MorphTargetName (Utilities|Struct|BreakStruct_MorphTargetSetup _array_element_7)) (Math|Float|MapRangeClamped (.DefaultValue (Utilities|Struct|BreakStruct_MorphTargetSetup _array_element_7)) (.x (.NormalizeToRange (Utilities|Struct|BreakStruct_MorphTargetSetup _array_element_7))) (.y (.NormalizeToRange (Utilities|Struct|BreakStruct_MorphTargetSetup _array_element_7))) -1.0 1.0) true))
            (for _array_element_8 (.ColorSchemes (Utilities|Struct|BreakStruct_SavedMeshes _array_element_2))
              (for _array_element_9 (.TargetMaterials (Utilities|Struct|BreakStruct_SavedColorSchemes _array_element_8))
                (bind _returnvalue_4 (Rendering|Material|CreateDynamicMaterialInstance _returnvalue_3 (.SlotIndex (Utilities|Struct|BreakStruct_MaterialSetup _array_element_9)) (.MaterialReference (Utilities|Struct|BreakStruct_MaterialSetup _array_element_9)) "None" :!class /Script/Engine.PrimitiveComponent))
                (for _array_element_10 (.Colors (Utilities|Struct|BreakStruct_SavedColorSchemes _array_element_8))
                  (if (.IsSelected (Utilities|Struct|BreakStruct_SavedColorSelection _array_element_10))
                    (Rendering|Material|SetVectorParameterValue _returnvalue_4 (.ParamaterName (Utilities|Struct|BreakStruct_MaterialSetup _array_element_9)) (.Color (Utilities|Struct|BreakStruct_SavedColorSelection _array_element_10)) :!class /Script/Engine.MaterialInstanceDynamic)))))))))
    ;[1 1 1] Add/Update Attachments
    (for _array_element_11 (LocalVariables|GetLocAvailableAttachments)
      (if (.IsSelected (Utilities|Struct|BreakStruct_SavedAttachments _array_element_11))
        (if (.UseSkeletalMesh (Utilities|Struct|BreakStruct_SavedAttachments _array_element_11))
          (bind _returnvalue_5 (AddComponent|AddSkeletalMeshComponent false))
          (Class|SkinnedMeshComponent|SetSkeletalMesh _returnvalue_5 (.SkeletalMesh (Utilities|Struct|BreakStruct_SavedAttachments _array_element_11)) true)
          (Transformation|AttachComponentToComponent _returnvalue_5 (Variables|Character|GetMesh) (.AttachToSocket (Utilities|Struct|BreakStruct_SavedAttachments _array_element_11)) "SnapToTarget" "SnapToTarget" "KeepRelative" true)
          (for _array_element_12 (.ColorSchemes (Utilities|Struct|BreakStruct_SavedAttachments _array_element_11))
            (for _array_element_13 (.TargetMaterials (Utilities|Struct|BreakStruct_SavedColorSchemes _array_element_12))
              (bind _returnvalue_6 (Rendering|Material|CreateDynamicMaterialInstance _returnvalue_5 (.SlotIndex (Utilities|Struct|BreakStruct_MaterialSetup _array_element_13)) (.MaterialReference (Utilities|Struct|BreakStruct_MaterialSetup _array_element_13)) "None" :!class /Script/Engine.PrimitiveComponent))
              (for _array_element_14 (.Colors (Utilities|Struct|BreakStruct_SavedColorSchemes _array_element_12))
                (if (.IsSelected (Utilities|Struct|BreakStruct_SavedColorSelection _array_element_14))
                  (Rendering|Material|SetVectorParameterValue _returnvalue_6 (.ParamaterName (Utilities|Struct|BreakStruct_MaterialSetup _array_element_13)) (.Color (Utilities|Struct|BreakStruct_SavedColorSelection _array_element_14)) :!class /Script/Engine.MaterialInstanceDynamic)))))
          (else
            (bind _returnvalue_7 (AddComponent|AddStaticMeshComponent false))
            (Components|StaticMesh|SetStaticMesh _returnvalue_7 (.StaticMesh (Utilities|Struct|BreakStruct_SavedAttachments _array_element_11)))
            (Transformation|AttachComponentToComponent _returnvalue_7 (Variables|Character|GetMesh) (.AttachToSocket (Utilities|Struct|BreakStruct_SavedAttachments _array_element_11)) "SnapToTarget" "SnapToTarget" "KeepRelative" true)
            (for _array_element_15 (.ColorSchemes (Utilities|Struct|BreakStruct_SavedAttachments _array_element_11))
              (for _array_element_16 (.TargetMaterials (Utilities|Struct|BreakStruct_SavedColorSchemes _array_element_15))
                (bind _returnvalue_8 (Rendering|Material|CreateDynamicMaterialInstance _returnvalue_7 (.SlotIndex (Utilities|Struct|BreakStruct_MaterialSetup _array_element_16)) (.MaterialReference (Utilities|Struct|BreakStruct_MaterialSetup _array_element_16)) "None" :!class /Script/Engine.PrimitiveComponent))
                (for _array_element_17 (.Colors (Utilities|Struct|BreakStruct_SavedColorSchemes _array_element_15))
                  (if (.IsSelected (Utilities|Struct|BreakStruct_SavedColorSelection _array_element_17))
                    (Rendering|Material|SetVectorParameterValue _returnvalue_8 (.ParamaterName (Utilities|Struct|BreakStruct_MaterialSetup _array_element_16)) (.Color (Utilities|Struct|BreakStruct_SavedColorSelection _array_element_17)) :!class /Script/Engine.MaterialInstanceDynamic))))))))))
  ;[1 1 1] Update Master Pose Component
  (for _array_element_18 (LocalVariables|GetSKMeshes)
    (Class|SkinnedMeshComponent|SetMasterPoseComponent _array_element_18 (Variables|Character|GetMesh) true)))