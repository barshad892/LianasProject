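; Player controller for the character customization demo, spawning and controlling a customization actor.
; On BeginPlay it spawns BP_CustomizationActor at a player start, blends the view to it and has the HUD create the customization menu.
; F toggles free look, showing or hiding the menu accordingly.
; Camera axis inputs drive the actor: vertical move and zoom only in free look, rotation in both modes.
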(event EventBeginPlay
  ;[1 1 1] For Demo Purposes I'll Spawn Right After Begin Play. You Can Call Anywhere You Like
  (CallFunction|SpawnCustomizationPawn))

(event EventSpawnCustomizationPawn
  ;[1 1 1] Spawn Customization Actor On "CharCustomization" Tagged Player Start
  (bind _returnvalue (Game|SpawnActorfromClass "/Game/DynamicCC/Blueprints/BP_CustomizationActor.BP_CustomizationActor_C" (Transformation|GetActorTransform (Class|GameModeBase|FindPlayerStart (Game|GetGameMode) self "CharCustomzation")) "AlwaysSpawn" 0 0))
  (Variables|Default|SetCustomizationActorReference _returnvalue)
  ;[1 1 1] Update View Target
  (Game|Player|SetViewTargetwithBlend (Variables|Default|GetCustomizationActorReference) 0.0 "VTBlend_Cubic" 0.0 true)
  ;[1 1 1] Create Customization Menu
  (Class|BPCCHUDInterface|CreateCustomizationMenu(Message) (HUD|GetHUD)))

(event Input|AxisEvents|InputAxisCameraMoveVertical
  (params (AxisValue :type Float%20%28single-precision%29))
  ;[1 1 1] Camera Move Inputs In Free Look
  (if (Variables|Default|GetIsInFreeLook?)
    (bind _returnvalue (CallFunction|GetCustomizationPawn))
    (Default|MoveCamera _returnvalue AxisValue)))

(event Input|AxisEvents|InputAxisCameraTurn
  (params (AxisValue :type Float%20%28single-precision%29))
  ;[1 1 1] Camera Move Inputs In Free Look
  (if (Variables|Default|GetIsInFreeLook?)
    _
    (else
      _))
  (bind _returnvalue (CallFunction|GetCustomizationPawn))
  (Default|RotateCamera _returnvalue AxisValue))

(event Input|AxisEvents|InputAxisCameraZoom
  (params (AxisValue :type Float%20%28single-precision%29))
  ;[1 1 1] Camera Move Inputs In Free Look
  (if (Variables|Default|GetIsInFreeLook?)
    (bind _returnvalue (CallFunction|GetCustomizationPawn))
    (Default|ZoomCamera _returnvalue AxisValue)))

(event Input|KeyboardEvents|F
  (params (Key :type Key%20Structure :default "None"))
  ;[1 1 1] Toggle Free Look
  (:Pressed
    (if (Variables|Default|GetIsInFreeLook?)
      (Variables|Default|SetIsInFreeLook? false)
      (else
        (Variables|Default|SetIsInFreeLook? true)))
    (Default|ToggleFreeLook (Variables|Default|GetCustomizationActorReference) (Variables|Default|GetIsInFreeLook?))
    (Class|BPCCHUDInterface|ToggleCustomizationMenu(Message) (HUD|GetHUD) (not (Variables|Default|GetIsInFreeLook?)))))

(fn ConstructionScript)

(fn RequestCustomizationPawn
  (return (Variables|Default|GetCustomizationActorReference)))