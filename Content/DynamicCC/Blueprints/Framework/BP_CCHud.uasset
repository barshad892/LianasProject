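; HUD Blueprint for the DynamicCC character customizer that owns the customization menu widget.
; CreateCustomizationMenu creates WB_CustomizerMain if it has none cached, adds it to the viewport, then sets game-and-UI input focused on it with a locked, visible cursor.
; ToggleCustomizationMenu forwards visibility to the widget, while RemoveCustomizationMenu is an empty stub.
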(event EventToggleCustomizationMenu
  (params (Visible :type Boolean))
  (Default|ToggleCustomizationMenu (Variables|Default|GetCustomizationMenuReference) Visible))

(event EventCreateCustomizationMenu
  (bind _returnvalue (Game|Player|GetOwningPlayerController))
  ;[1 1 1] Create Customization Menu And Add To Viewport
  (Variables|Default|GetCustomizationMenuReference
    (:then
      _)
    (:else
      (bind _returnvalue_2 (UserInterface|CreateWidget "/Game/DynamicCC/UserInterface/WB_CustomizerMain.WB_CustomizerMain_C"))
      (Variables|Default|SetCustomizationMenuReference _returnvalue_2)))
  (UserInterface|Viewport|AddtoViewport (Variables|Default|GetCustomizationMenuReference) 0)
  ;[1 1 1] Set Input Mode
  (Input|SetInputModeGameandUI _returnvalue (Variables|Default|GetCustomizationMenuReference) "LockAlways" false)
  (Variables|/Script/Engine.PlayerController|SetbShowMouseCursor _returnvalue true))

(event EventRemoveCustomizationMenu)

(fn ConstructionScript)