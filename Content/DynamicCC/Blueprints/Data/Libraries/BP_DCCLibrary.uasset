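; Blueprint function library for the DynamicCC system, providing shared helpers for pawn access and UI grid layout.
; GetCustomizationPawn returns the customization pawn by sending a request message to the first player controller, without a cast in the function.
; GenerateGrid adds a widget to a Uniform Grid and derives its row and column from the child count and column count, filling row by row.
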(fn GetCustomizationPawn
  (bind _returnvalue (Class|BPCCPlayerControllerInterface|RequestCustomizationPawn(Message) (Game|GetPlayerController 0)))
  (return _returnvalue))

(fn GenerateGrid
  (params (Grid :type Uniform%20Grid%20Panel%20Object%20Reference) (Content :type Widget%20Object%20Reference) (Column :type Integer))
  (bind _returnvalue (Class|PanelWidget|GetChildrenCount Grid))
  (bind _returnvalue_2 (- _returnvalue 1))
  (bind _returnvalue_3 (Class|UniformGridPanel|AddChildtoUniformGrid Grid Content))
  (Class|UniformGridSlot|SetRow _returnvalue_3 (/ _returnvalue_2 Column))
  (Class|UniformGridSlot|SetColumn _returnvalue_3 (Math|Integer|%(Integer) _returnvalue_2 Column)))