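; Inventory item actor that the player can take, store and inspect in 3D.
; It binds to the character's pickup event, then adds its item struct to the HUD inventory, hides the mesh, restores player control and shows a timed message.
; Inventory menu clicks show or hide the mesh before the camera.
; Holding left mouse rotates it through a sphere pivot, which is reset by detaching and reattaching the mesh to avoid gimbal lock.
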(event Custom|PickupItem_Event_0
  (bind _mycharacter (Variables|Default|GetMyCharacter))
  (bind _gamehudwidgetue (Variables|/Game/CV3rdPersInterface/Blueprints/ThirdPersonCharacter.ThirdPersonCharacter_C|GetGameHUDWidgetUE _mycharacter))
  ;[1 1 1] Pick up and Add Item to Inventory UE - message from Examine Menu button 'Take'
  (Variables|Default|SetHaveItemInHand2 false)
  (Variables|Default|SetItemInInventory true)
  (Utilities|Array|AddUnique (Variables|/Game/CV3rdPersInterface/Blueprints/Widgets/BPW_INVExamine.BPW_INVExamine_C|GetInventoryUE _gamehudwidgetue) (Variables|Default|GetItemInfoUE))
  ;;[1 1 1] Hide InvItem while in Inventory until called for
  (Development|SetHiddeninGame (Variables|Default|GetInvMesh) true false)
  ;[1 1 1] From here GO TO REHIDE Examine Menu
  ;;[1 1 1] Resets inventory items, and re-arranges them according to empty sockets
  (Default|RefreshInventory _gamehudwidgetue)
  ;;[1 1 1] Unfreeze player and give nagivation control back to mouse
  (Class|BPIFreezePlayer|FreezePlayer(Message) (Game|GetPlayerCharacter 0) false)
  (Input|SetInputModeGameOnly (Game|GetPlayerController 0))
  (Variables|/Script/Engine.PlayerController|SetbShowMouseCursor (Game|GetPlayerController 0) false)
  (Viewport|RemoveAllWidgets)
  ;;[1 1 1] Sends message to FPC that an object has been taken
  (Class|BPIInvActor2FPC|ObjectTaken(Message) (Game|GetPlayerCharacter 0) true)
  ;[1 1 1] UMG Message to player about taking the object into inventory
  (bind _returnvalue (UserInterface|CreateWidget "/Game/CV3rdPersInterface/Blueprints/Widgets/BPW_DialogBox.BPW_DialogBox_C"))
  (bind _output_get (Variables|Default|SetAddItemToInvMess _returnvalue))
  (Class|BPIDialogTxtMessage|DialogTxtMessage(Message) _output_get (Utilities|Text|ToText(String) (Utilities|String|Append (Utilities|String|Append "You have added " (Utilities|String|ToString(Text) (Variables|Default|GetInvActorTextFordialog))) " to your inventory.")))
  (if (Variables|Default|GetAlreadyOnScreen)
    ;;[1 1 1] Add Message to screen, allow 3 seconds for fade animation, then remove from screen
    (Viewport|RemoveAllWidgets)
    (else
      (UserInterface|Viewport|AddtoViewport (Variables|Default|GetAddItemToInvMess) 0)
      (Variables|Default|SetAlreadyOnScreen true)
      (Utilities|FlowControl|Delay 3.0)
      (Widget|RemovefromParent (Variables|Default|GetAddItemToInvMess))))
  (Variables|Default|SetAlreadyOnScreen false))

(event EventDestroyInvActor
  (params (DestroyInvActor :type Boolean))
  ;[1 1 1] From FirstPersonChar - destroy inventory actor
  (if DestroyInvActor
    (Actor|DestroyActor)))

(event EventBeginPlay
  (bind _iteminfoue (Variables|Default|GetItemInfoUE))
  (bind (_itemname _itemdescription1 _invdropactorclass _invmesh _inviconimage _itemactor _inventoryclass _isusable) (Utilities|Struct|BreakBS_InvInfoStruct _iteminfoue))
  ;[1 1 1] Event Begin Play
  ;;[1 1 1] Get all the inventory item classes and put into an array for later use by this BP
  (bind _outactors (Actor|GetAllActorsOfClass _inventoryclass))
  (for _array_element _outactors
    (Utilities|Struct|SetmembersinBS_InvInfoStruct (Utilities|Struct|MakeBS_InvInfoStruct _itemname _itemdescription1 _invdropactorclass _invmesh _inviconimage _itemactor _inventoryclass _isusable) "" "" 0 0 0 0 0 false)
    ;;[1 1 1] Launches Event Pickupitem below
    (bind _asthird_person_character (Utilities|Casting|CastToThirdPersonCharacter (Game|GetPlayerCharacter 0))
      (:then
        (bind _output_get (Variables|Default|SetMyCharacter _asthird_person_character))
        (EventDispatchers|BindEventtoPickUpItem _output_get (delegate Custom|PickupItem_Event_0)))
      (:CastFailed
        (Development|PrintString "Cant failed due to being unable to find a valid First Person Character"))))
  (Utilities|Struct|SetmembersinBS_InvInfoStruct (Utilities|Struct|MakeBS_InvInfoStruct _itemname _itemdescription1 _invdropactorclass _invmesh _inviconimage _itemactor _inventoryclass _isusable) "" "" 0 0 0 0 0 false)
  (bind _asthird_person_character_2 (Utilities|Casting|CastToThirdPersonCharacter (Game|GetPlayerCharacter 0))
    (:then
      (bind _output_get_2 (Variables|Default|SetMyCharacter _asthird_person_character_2))
      (EventDispatchers|BindEventtoPickUpItem _output_get_2 (delegate Custom|PickupItem_Event_0)))
    (:CastFailed
      (Development|PrintString "Cant failed due to being unable to find a valid First Person Character"))))

(event EventInvEx2InvActor
  (params (HideMesh :type Boolean))
  (bind _returnvalue (Game|GetPlayerCameraManager 0))
  (bind _returnvalue_2 (Game|GetPlayerController 0))
  (bind _invmesh (Variables|Default|GetInvMesh))
  (bind (_outlocation _outrotation) (Actor|GetActorEyesViewPoint _returnvalue))
  ;[1 1 1] From InvExamine UMG widget - item in inventory list was clicked on
  ;;[1 1 1] Message sent from Inventory Menu screen when an icon is clicked on
  (Variables|Default|SetCharacterEyesLocation _outrotation)
  (Variables|Default|SetNewEyesLocation (+ _outlocation (Math|Vector|RotateVector "20.000000,1.500000,1.000000" _outrotation)))
  (if HideMesh
    (Development|SetHiddeninGame _invmesh true false)
    (else
      (Development|SetHiddeninGame _invmesh false false)
      ;;[1 1 1] Put InvMesh at location of player Eyes
      (Transformation|SetWorldLocationAndRotation (Variables|Default|GetInvMesh) (Variables|Default|GetNewEyesLocation) (Variables|Default|GetCharacterEyesLocation) false false)
      ;;[1 1 1] Enables input from keyboard and mouse to interact with level AND UI at same time to rotate 3D items
      (Input|EnableInput _returnvalue_2)
      (Input|SetInputModeGameandUI _returnvalue_2 0 "DoNotLock" true)
      (Variables|Default|SetHaveItemInHand2 true))))

(event Input|AxisEvents|InputAxisTurn
  (params (AxisValue :type Float%20%28single-precision%29))
  ;[1 1 1] Rotate Object when viewing inside of Inventory - each time Turn or Tumble happens, the SpherePivot is reset, and InvMesh is reparented so moving mouse always has same effect.
  ;;[1 1 1] If false return mouse navigation control back to the character
)

(event Input|AxisEvents|InputAxisLookUp
  (params (AxisValue :type Float%20%28single-precision%29))
  ;[1 1 1] Rotate Object when viewing inside of Inventory - each time Turn or Tumble happens, the SpherePivot is reset, and InvMesh is reparented so moving mouse always has same effect.
  ;;[1 1 1] If false return mouse navigation control back to the character
)

(event Input|AxisEvents|InputAxisTurnObject
  (params (AxisValue :type Float%20%28single-precision%29))
  (bind _returnvalue (Game|GetPlayerCharacter 0))
  ;[1 1 1] Rotate Object when viewing inside of Inventory - each time Turn or Tumble happens, the SpherePivot is reset, and InvMesh is reparented so moving mouse always has same effect.
  ;;[1 1 1] If the item is in hand, rotate it, if not, return control back to player controller
  (if (Variables|Default|GetHaveItemInHand2)
    ;[1 1 1] Check to see if Left Mouse Button has been clicked and is held down to determine if the Inventory item should be rotating during mouse move or not
    (if (Game|Player|IsInputKeyDown (Game|GetPlayerController 0) "LeftMouseButton")
      ;[1 1 1] Attach InvMesh to the SpherePivotINV and will inherit its rotation
      (Class|SceneComponent|Attachto (Variables|Default|GetInvMesh) (Variables|Default|GetSpherePivotINV) "None" "KeepWorldPosition" true)
      ;[1 1 1] Rotates Yaw (turn left to right).
      ;;[1 1 1] Rotates SpherePivotINV which inturn rotates its child "InvMesh
      (Transformation|AddLocalRotation (Variables|Default|GetSpherePivotINV) (Math|Rotator|MakeRotator 0.0 0.0 (* (* (stale Input|AxisEvents|InputAxisTurn AxisValue) -1.0) 4.0)) false false)
      (else
        ;[1 1 1] Detaches from Sphere parent, Resents Parents Rotate,then reattaches, to avoid gimble lock
        (Class|SceneComponent|DetachfromParent (Variables|Default|GetInvMesh) true true)
        (Transformation|SetWorldLocationAndRotation (Variables|Default|GetSpherePivotINV) (Variables|Default|GetNewEyesLocation) (Variables|Default|GetCharacterEyesLocation) false false)
        (Class|SceneComponent|Attachto (Variables|Default|GetInvMesh) (Variables|Default|GetSpherePivotINV) "None" "KeepWorldPosition" false)))
    (else
      ;;[1 1 1] If false return mouse navigation control back to the character
      (Pawn|Input|AddControllerYawInput _returnvalue (stale Input|AxisEvents|InputAxisTurn AxisValue))
      (Pawn|Input|AddControllerPitchInput _returnvalue (stale Input|AxisEvents|InputAxisLookUp AxisValue)))))

(event Input|AxisEvents|InputAxisTumbleObject
  (params (AxisValue :type Float%20%28single-precision%29))
  ;[1 1 1] Rotate Object when viewing inside of Inventory - each time Turn or Tumble happens, the SpherePivot is reset, and InvMesh is reparented so moving mouse always has same effect.
  ;;[1 1 1] If the item is in hand, rotate it, if not, return control back to player controller
  (if (Variables|Default|GetHaveItemInHand2)
    ;;[1 1 1] Rotates Pitch (up and down mouse movement) up is tip forward down is tip back
    (if (Game|Player|IsInputKeyDown (Game|GetPlayerController 0) "LeftMouseButton")
      ;;;[1 1 1] Parent InvMesh to SpherePivotINV for rotating
      (Class|SceneComponent|Attachto (Variables|Default|GetInvMesh) (Variables|Default|GetSpherePivotINV) "None" "KeepWorldPosition" false)
      (Transformation|AddLocalRotation (Variables|Default|GetSpherePivotINV) (Math|Rotator|MakeRotator 0.0 (* (* (stale Input|AxisEvents|InputAxisLookUp AxisValue) 1.0) 4.0) 0.0) false false)
      (else
        ;;;[1 1 1] Detach InvMesh from SpherePivotINV temporarily, Reset SpherePivotINV Rotation values, then ReParent InvMesh to SpherePivotINV - this resets the rotation values to eliminate gimble lock and reverse rotating
        (Class|SceneComponent|DetachfromParent (Variables|Default|GetInvMesh) true true)
        (Transformation|SetWorldLocationAndRotation (Variables|Default|GetSpherePivotINV) (Variables|Default|GetNewEyesLocation) (Variables|Default|GetCharacterEyesLocation) false false)
        (Class|SceneComponent|Attachto (Variables|Default|GetInvMesh) (Variables|Default|GetSpherePivotINV) "None" "KeepWorldPosition" false)))
    (else
      ;;[1 1 1] If false return mouse navigation control back to the character
      (Pawn|Input|AddControllerPitchInput (Game|GetPlayerCharacter 0) (stale Input|AxisEvents|InputAxisLookUp AxisValue)))))

(fn ConstructionScript)

(fn Destroyme
  (return false))

(fn UpdateInvInfo
  (return false))