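; Fire extinguisher pickup, a child Blueprint that supplies this item's examine text and inventory data to its parent pickup class.
; Its construction script sets the mesh's custom depth stencil value according to whether the item is takable, then runs the parent script.
; The OnExamine override fills in the description, inventory and drop classes, item info struct and takable state from its own variables, then returns the parent's result.
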(fn ConstructionScript
  (bind _pickupmesh (Variables|Default|GetPickupMesh))
  (if (Utilities|Enum|Equal(Enum) (Variables|Default|GetThisTakableOrNot) "NewEnumerator0")
    (Rendering|SetCustomDepthStencilValue _pickupmesh 252)
    (else
      (Rendering|SetCustomDepthStencilValue _pickupmesh 254)))
  (|CallParentFunction))

(fn OnExamine
  (params (Character :type Third%20Person%20Character%20Object%20Reference))
  (bind _thisinvdropactorclass (Variables|Default|GetThisInvDropActorClass))
  (bind _thisinventoryclass (Variables|Default|GetThisInventoryClass))
  (Variables|Default|SetItemDescription "This is a very used fire extinguisher. The tank is very old and looks like it has seen some action. 
 
However - the handles and hose have recently been replaced and looks brand new. The gauge shows a full tank.")
  (Variables|Default|SetInventoryClass _thisinventoryclass)
  (Variables|Default|SetClassOfBP _thisinvdropactorclass)
  (Variables|Default|SetItemInfo (Utilities|Struct|MakeBS_InvInfoStruct (Variables|Default|GetThisItemName) "" _thisinvdropactorclass 0 (Variables|Default|GetThisInvIconImage) 0 _thisinventoryclass (Variables|Default|GetThisIsUsable)))
  (Variables|Default|SetTakableOrNot (Variables|Default|GetThisTakableOrNot))
  (bind _success (|CallParentFunction 0))
  (return _success))