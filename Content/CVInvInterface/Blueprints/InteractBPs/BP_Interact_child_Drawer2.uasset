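; BP_Interact_child_Drawer2 is an interactable locked drawer that opens and closes through a Level Sequence.
; On interact, an unlocked drawer alternates forward and reverse playback via a FlipFlop.
; While locked, an empty inventory shows a timed "locked" dialog widget; otherwise it compares every world BP_InventoryActor's ItemID against KeymasterID.
; A match permanently sets the unlocked flag and toggles the drawer, while each mismatch triggers the dialog.
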(event EventOnInteract
  (params (Character :type First%20Person%20Character%20Object%20Reference))
  ;[1 1 1] Locked Drawer - check to see if you have the KEY in your INVENTORY - if NOT say that its locked. If YES unlock and set Drawer is unlocked Var for next time. so player can get rid of Key.
  (if (Variables|Default|GetDrawerIsUnlocked)
    (Utilities|FlowControl|FlipFlop :!label _label
      (:A
        (bind _returnvalue (Sequencer|Player|CreateLevelSequencePlayer "/Game/CVInvInterface/Sequences/S_Drawer2Sequence.S_Drawer2Sequence"))
        (Audio|Components|Audio|Play _returnvalue))
      (:B
        (Class|LevelSequencePlayer|PlayReverse _returnvalue)))
    (elif (< (Utilities|Array|Length (Variables|/Game/CVInvInterface/Blueprints/Widgets/BPW_INVExamine.BPW_INVExamine_C|GetInventoryUE (Variables|/Game/CVInvInterface/Blueprints/FirstPersonCharacter.FirstPersonCharacter_C|GetGameHUDWidgetUE Character))) 1)
      ;[1 1 1] UMG Dialog Box for locked drawer
      (bind _returnvalue_2 (UserInterface|CreateWidget "/Game/CVInvInterface/Blueprints/Widgets/BPW_DialogBox.BPW_DialogBox_C" :!label _label_2))
      (Class|BPIDialogTxtMessage|DialogTxtMessage(Message) _returnvalue_2 (Variables|Default|GetTextForDialog))
      (if (Variables|Default|GetAlreadyViewable)
        (Viewport|RemoveAllWidgets)
        (else
          (UserInterface|Viewport|AddtoViewport _returnvalue_2 0)
          (Variables|Default|SetAlreadyViewable true)
          (Utilities|FlowControl|Delay 3.0)
          (Widget|RemovefromParent _returnvalue_2)))
      (Variables|Default|SetAlreadyViewable false)
      (else
        (bind _outactors (Actor|GetAllActorsOfClass "/Game/CVInvInterface/Blueprints/InventoryActorBPS/BP_InventoryActor.BP_InventoryActor_C"))
        (for _array_element _outactors
          (if (== (Variables|/Game/CVInvInterface/Blueprints/InventoryActorBPS/BP_InventoryActor.BP_InventoryActor_C|GetItemID _array_element) (Variables|Default|GetKeymasterID))
            ;;[1 1 1] If the Item ID matches -un lock the drawer
            (Variables|Default|SetDrawerIsUnlocked true)
            (goto _label)
            (else
              (goto _label_2))))))))

(fn ConstructionScript
  (|CallParentFunction))