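; BP_InventoryActor_Child_FireExtinguisher is the inventory item for a usable fire extinguisher, setting its description and item info in construction.
; On use, it spawns BP_FireExtUSE in front of the player's eyes, attaches it to the camera manager, cancels the inventory and briefly shows a how-to-stop dialog.
; Button press and release send activate and deactivate messages to the spawned extinguisher, found by class.
; TurnHandHeldOff destroys it when the inventory reopens.
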(event EventUseInvActor
  (params (UseInvActorBool :type Boolean))
  (bind _returnvalue (Game|GetPlayerCharacter 0))
  (bind (_outlocation _outrotation) (Actor|GetActorEyesViewPoint _returnvalue))
  ;[1 1 1] Message from FirstPersonCharacter
  ;[1 1 1] Get location of player and POV then SPAWN the actor that you want to use.
  (bind _returnvalue_2 (Game|SpawnActorfromClass "/Game/CVInvInterface/Blueprints/HandHeldBPs/BP_FireExtUSE.BP_FireExtUSE_C" (Math|Transform|MakeTransform (+ _outlocation (Math|Vector|RotateVector "20.000000,0.000000,-6.000000" _outrotation)) _outrotation "1.000000,1.000000,1.000000") "AdjustIfPossibleButDontSpawnIfColliding" 0 0))
  (Class|Actor|AttachRootComponenttoActor _returnvalue_2 (Game|GetPlayerCameraManager 0) "None" "KeepWorldPosition" true)
  (Class|BPICancelInventory|CancelInventory(Message) (Game|GetPlayerCharacter 0) false)
  ;[1 1 1] Dialog Box
  (Variables|Default|SetAlreadyOnScreen false)
  (bind _returnvalue_3 (UserInterface|CreateWidget "/Game/CVInvInterface/Blueprints/Widgets/BPW_DialogBox.BPW_DialogBox_C"))
  (Class|BPIDialogTxtMessage|DialogTxtMessage(Message) _returnvalue_3 (Utilities|Text|ToText(String) (Utilities|String|Append (Utilities|String|Append "Press the \"I\" key to stop using  " (Utilities|String|ToString(Text) (Variables|Default|GetInvActorTextFordialog))) " and return to your inventory.")))
  (if (Variables|Default|GetAlreadyOnScreen)
    (Viewport|RemoveAllWidgets)
    (else
      (UserInterface|Viewport|AddtoViewport _returnvalue_3 0)
      (Variables|Default|SetAlreadyOnScreen true)
      (Utilities|FlowControl|Delay 3.0)
      (Widget|RemovefromParent _returnvalue_3)))
  (Variables|Default|SetAlreadyOnScreen false))

(event EventTurnHandHeldOff
  (params (success :type Boolean))
  ;[1 1 1] "I" key was pressed to open inventory screen and STOP using item
  (Actor|DestroyActor (stale EventUseInvActor _returnvalue_2)))

(event EventUseInvActorButtonPress
  ;[1 1 1] Mouse Clicks - Down and Release actions
  (bind _outactors (Actor|GetAllActorsOfClass "/Game/CVInvInterface/Blueprints/HandHeldBPs/BP_FireExtUSE.BP_FireExtUSE_C"))
  (Class|BPIActivateItem|ActivateItem(Message) _outactors false))

(event EventUseInvActorButtonRelease
  ;[1 1 1] Mouse Clicks - Down and Release actions
  (bind _outactors (Actor|GetAllActorsOfClass "/Game/CVInvInterface/Blueprints/HandHeldBPs/BP_FireExtUSE.BP_FireExtUSE_C"))
  (Class|BPIActivateItem|DeactivateItem(Message) _outactors false))

(fn ConstructionScript
  (bind _output_get (Variables|Default|SetNEWItemDescription "This is a very used fire extinguisher. The tank is very old and looks like it has seen some action. 
 
However - the handles and hose have recently been replaced and looks brand new. The gauge shows a full tank."))
  (Utilities|Struct|SetmembersinBS_InvInfoStruct (Variables|Default|GetItemInfoUE) (Variables|Default|GetMyItemName) _output_get (Variables|Default|GetMyInvDropActorClass) 0 (Variables|Default|GetMyInvIconImage) 0 (Variables|Default|GetMyInventoryClass) (Variables|Default|GetMyIsUsable))
  ;[1 1 1] This appears when adding an item to your inventory. It will tell you "You have added (YourItemName) to your inventory"
  (Variables|Default|SetInvActorTextFordialog "a used fire extinguisher")
  (|CallParentFunction))