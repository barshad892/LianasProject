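; Beachball inventory item actor, a child Blueprint of an inventory actor base, holding the item's data for the inventory system.
; Its Construction Script writes name, placeholder description, icon, drop actor class, inventory class and usable flag into the item info struct, sets the dialog text to "a beachball", then calls the parent.
; UpdateInvInfo just defers to the parent, and the Event Graph's setup nodes never run.
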(fn ConstructionScript
  (bind _output_get (Variables|Default|SetNEWItemDescription "Relace this text. This text appears on the Inventory screen when opening the Inventory by pressing the \"I\" key. 
 
Use SHIFT-RETURN to do a line/paragraph break. 
 
This text is unique to the Inventory screen. You can have the same or different information in the description area after you take the item into your inventory."))
  (Utilities|Struct|SetmembersinBS_InvInfoStruct (Variables|Default|GetItemInfoUE) (Variables|Default|GetMyItemName) _output_get (Variables|Default|GetMyInvDropActorClass) 0 (Variables|Default|GetMyInvIconImage) 0 (Variables|Default|GetMyInventoryClass) (Variables|Default|GetMyIsUsable))
  (Variables|Default|SetInvActorTextFordialog "a beachball")
  (|CallParentFunction))

(fn UpdateInvInfo
  (bind _succes (|CallParentFunction))
  (return _succes))