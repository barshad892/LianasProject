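; Interactable locked drawer that opens and closes once unlocked with a matching key item.
; On interact while locked, it compares each BP_InventoryActor's ItemID to KeymasterID, and non-matches trigger a timed BPW_DialogBox message.
; A match sets DrawerIsUnlocked, so the key is not checked again.
; Toggling plays the S_Drawer2Sequence level sequence forward to open, then reverses that player to close.
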(event EventOnInteract
  (params (Character :type Third%20Person%20Character%20Object%20Reference))
  ;[1 1 1] Locked Drawer - check to see if you have the KEY in your INVENTORY - if NOT say that its locked. If YES unlock and set Drawer is unlocked Var for next time. so player can get rid of Key.
  (if (Variables|Default|GetDrawerIsUnlocked)
    (if (Variables|Default|GetDrawerIsOpen) :!label _label
      (Variables|Default|SetDrawerIsOpen false)
      (Class|LevelSequencePlayer|PlayReverse (Variables|/Script/LevelSequence.LevelSequenceActor|GetSequencePlayer (stale _outactor)))
      (else
        (Variables|Default|SetDrawerIsOpen true)
        (bind _outactor (Sequencer|Player|CreateLevelSequencePlayer "/Game/Quest2_BLueprints/CV3rdPersInterface/Sequences/S_Drawer2Sequence.S_Drawer2Sequence"))
        (Audio|Components|Audio|Play (Variables|/Script/LevelSequence.LevelSequenceActor|GetSequencePlayer _outactor))))
    (else
      (bind _outactors (Actor|GetAllActorsOfClass "/Game/Quest2_BLueprints/CV3rdPersInterface/Blueprints/InventoryActorBPS/BP_InventoryActor.BP_InventoryActor_C"))
      (for _array_element _outactors
        (if (== (Variables|/Game/Quest2_BLueprints/CV3rdPersInterface/Blueprints/InventoryActorBPS/BP_InventoryActor.BP_InventoryActor_C|GetItemID _array_element) (Variables|Default|GetKeymasterID))
          ;;[1 1 1] If the Item ID matches -un lock the drawer
          (Variables|Default|SetDrawerIsUnlocked true)
          (goto _label)
          (else
            ;[1 1 1] UMG Dialog Box for locked drawer
            (bind _returnvalue (UserInterface|CreateWidget "/Game/Quest2_BLueprints/CV3rdPersInterface/Blueprints/Widgets/BPW_DialogBox.BPW_DialogBox_C"))
            (Class|BPIDialogTxtMessage|DialogTxtMessage(Message) _returnvalue (Variables|Default|GetTextForDialog))
            (if (Variables|Default|GetAlreadyViewable)
              (Viewport|RemoveAllWidgets)
              (else
                (UserInterface|Viewport|AddtoViewport _returnvalue 0)
                (Variables|Default|SetAlreadyViewable true)
                (Utilities|FlowControl|Delay 3.0)
                (Widget|RemovefromParent _returnvalue)))
            (Variables|Default|SetAlreadyViewable false))))
      (if (== (Variables|/Game/Quest2_BLueprints/CV3rdPersInterface/Blueprints/InventoryActorBPS/BP_InventoryActor.BP_InventoryActor_C|GetItemID _array_element) (Variables|Default|GetKeymasterID))
        (Variables|Default|SetDrawerIsUnlocked true)
        (goto _label)
        (else
          (bind _returnvalue_2 (UserInterface|CreateWidget "/Game/Quest2_BLueprints/CV3rdPersInterface/Blueprints/Widgets/BPW_DialogBox.BPW_DialogBox_C"))
          (Class|BPIDialogTxtMessage|DialogTxtMessage(Message) _returnvalue_2 (Variables|Default|GetTextForDialog))
          (if (Variables|Default|GetAlreadyViewable)
            (Viewport|RemoveAllWidgets)
            (else
              (UserInterface|Viewport|AddtoViewport _returnvalue_2 0)
              (Variables|Default|SetAlreadyViewable true)
              (Utilities|FlowControl|Delay 3.0)
              (Widget|RemovefromParent _returnvalue_2)))
          (Variables|Default|SetAlreadyViewable false))))))

(fn ConstructionScript
  (|CallParentFunction))