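; Dinosaur egg pickup, a child Blueprint that supplies the egg's examine description and inventory data.
; Actor overlap shows an Item_Found prompt widget; ending overlap or clicking left mouse removes it and sets the player's objective to a Tab-to-use hint.
; The construction script picks the mesh's custom depth stencil value from the takable setting.
; OnExamine fills the item info struct from instance variables, then calls the parent implementation.
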(event Collision|EventActorBeginOverlap
  (params (OtherActor :type Actor%20Object%20Reference))
  ;[1 1 1] Show widget text of (Press "F" to Pickup Key)
  (bind _returnvalue (UserInterface|CreateWidget "/Game/Quest2_BLueprints/widgets/Item_Found.Item_Found_C" (Game|GetPlayerController 0)))
  (bind _output_get (Variables|Default|Setitem_foundWidget _returnvalue))
  (UserInterface|Viewport|AddtoViewport _output_get 0))

(event Collision|EventActorEndOverlap
  (params (OtherActor :type Actor%20Object%20Reference))
  ;[1 1 1] Remove text as he pickup the key
  (Widget|GetAllWidgetsOfClass "/Game/Quest2_BLueprints/widgets/Item_Found.Item_Found_C" true)
  (bind _asitem_found (Utilities|Casting|CastToItem_Found (Variables|Default|Getitem_foundWidget)))
  (Widget|RemovefromParent _asitem_found)
  (bind _asthird_person_character_1 (Utilities|Casting|CastToThirdPersonCharacter1 (Game|GetPlayerCharacter 0)))
  (Variables|/Game/Quest2_BLueprints/ThirdPersonCharacter1.ThirdPersonCharacter1_C|SetPlayerObjective _asthird_person_character_1 "To use the item, Press \"Tab\""))

(event Input|MouseEvents|LeftMouseButton
  (params (Key :type Key%20Structure :default "None"))
  (:Pressed
    ;[1 1 1] Remove text as he pickup the key
    (Widget|GetAllWidgetsOfClass "/Game/Quest2_BLueprints/widgets/Item_Found.Item_Found_C" true)
    (bind _asitem_found (Utilities|Casting|CastToItem_Found (Variables|Default|Getitem_foundWidget)))
    (Widget|RemovefromParent _asitem_found)
    (bind _asthird_person_character_1 (Utilities|Casting|CastToThirdPersonCharacter1 (Game|GetPlayerCharacter 0)))
    (Variables|/Game/Quest2_BLueprints/ThirdPersonCharacter1.ThirdPersonCharacter1_C|SetPlayerObjective _asthird_person_character_1 "To use the item, Press \"Tab\"")))

(fn ConstructionScript
  (bind _pickupmesh (Variables|Default|GetPickupMesh))
  (if (Utilities|Enum|Equal(Enum) (Variables|Default|GetThisTakableOrNot) "NewEnumerator0")
    (Rendering|SetCustomDepthStencilValue _pickupmesh 252)
    (else
      (Rendering|SetCustomDepthStencilValue _pickupmesh 254)))
  (|CallParentFunction))

(fn OnExamine
  (params (Character :type Third%20Person%20Character%20Quest%202%20Object%20Reference))
  (bind _thisinvdropactorclass (Variables|Default|GetThisInvDropActorClass))
  (bind _thisinventoryclass (Variables|Default|GetThisInventoryClass))
  (Variables|Default|SetItemDescription "This appears to be a fully intact and recently paid dinosaur egg. It is warm to the touch and a bit slimy. ")
  (Variables|Default|SetInventoryClass _thisinventoryclass)
  (Variables|Default|SetClassOfBP _thisinvdropactorclass)
  (Variables|Default|SetItemInfo (Utilities|Struct|MakeBS_InvInfoStruct (Variables|Default|GetThisItemName) "" _thisinvdropactorclass 0 (Variables|Default|GetThisInvIconImage) 0 _thisinventoryclass (Variables|Default|GetThisIsUsable)))
  (Variables|Default|SetTakableOrNot (Variables|Default|GetThisTakableOrNot))
  (bind _success (|CallParentFunction 0))
  (return _success))