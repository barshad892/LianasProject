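; Base pickup actor that highlights on focus via custom depth and can be examined up close.
; Examining a still item freezes the player, hides the mesh, spawns its inventory actor before the camera and opens a takable or examine-only widget.
; Mouse drag rotates it on a sphere pivot, reset on release to avoid gimbal lock.
; Putting back restores the pickup; dropping destroys it and spawns a new one in front of the player.
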(event Custom|PutTheItemBack
  (bind _returnvalue (Game|GetPlayerController 0))
  ;[1 0 0.09067] Put Object Back from Examine menu
  (if (Variables|Default|GetbHaveItemInHand)
    (Variables|Default|SetbHaveItemInHand false)
    ;;[1 1 1] UnFeeze player to give mouse control back to player character
    (Class|BPIFreezePlayer|FreezePlayer(Message) (Game|GetPlayerCharacter 0) false)
    ;;[1 1 1] Destroy the current Inventory Mesh displayed
    (Actor|DestroyActor (Variables|Default|GetBPInventoryActor))
    ;;[1 1 1] Re-show (unhide) Pickup Mesh
    (Development|SetHiddeninGame (Variables|Default|GetPickupMesh) false false)
    ;[1 1 1] Remove Examine Menu UMG from screen
    (Variables|/Script/Engine.PlayerController|SetbShowMouseCursor (Game|GetPlayerController 0) false)
    ;;[1 1 1] If Examine Menu is open, close it
    (Utilities|IsValid (Variables|Default|GetExamineMenu)
      (:Is%20Valid
        (Widget|RemovefromParent (Variables|Default|GetExamineMenu))
        ;;[1 1 1] If Examine Only Menu is open, close it
        (Utilities|IsValid (Variables|Default|GetExamineOnlyMenu)
          (:Is%20Valid
            (Widget|RemovefromParent (Variables|Default|GetExamineOnlyMenu) :!label _label))
          (:Is%20Not%20Valid
            _)))
      (:Is%20Not%20Valid
        (goto _label)))
    ;;[1 1 1] Set input mode back to Game Only
    (Input|SetInputModeGameOnly _returnvalue)
    ;;[1 1 1] Turn Cross Hairs back on after closing Examine Menus
    (bind _asfirst_person_hud (Utilities|Casting|CastToFirstPersonHUD (HUD|GetHUD _returnvalue))
      (:then
        (Variables|/Game/Quest2_BLueprints/CVInvInterface/Blueprints/FirstPersonHUD.FirstPersonHUD_C|SetShowCrossHairs _asfirst_person_hud true))
      (:CastFailed
        (Development|PrintString "Cast failed due to not finding a valid HUD within Player Controller")))))

(event Custom|DropItemFromMenu
  (bind _returnvalue (Game|GetPlayerController 0))
  (bind _returnvalue_2 (Game|Player|GetPlayerPawn 0))
  (bind _returnvalue_3 (Pawn|GetControlRotation _returnvalue_2 :!class /Script/Engine.Pawn))
  ;[1 0 0.09067] Drop action is pressed from Examine Menu
  (if (Variables|Default|GetbHaveItemInHand)
    (Variables|Default|SetbHaveItemInHand false)
    (Physics|SetSimulatePhysics (Variables|Default|GetPickupMesh) true)
    ;;[1 1 1] Return movement control to Player Character
    (Class|BPIFreezePlayer|FreezePlayer(Message) (Game|GetPlayerCharacter 0) false)
    ;;[1 1 1] Destroy current item being examined up close
    (Actor|DestroyActor (Variables|Default|GetBPInventoryActor))
    ;;[1 1 1] Destroy Original Pickup Actor at its old location before pickup
    (Development|SetHiddeninGame (Variables|Default|GetPickupMesh) false false)
    (Actor|DestroyActor)
    ;[1 1 1] Determine location of character to drop item in front of
    ;;[1 1 1] Spawn New Pickup Item at Drop Location
    (bind _output_get (Variables|Default|SetDropSpawnLocation (Math|Transform|MakeTransform (+ (+ (Transformation|GetActorLocation _returnvalue_2) (Math|Vector|RotateVector "150.000000,0.000000,0.000000" _returnvalue_3)) "0.000000,0.000000,150.000000") _returnvalue_3 "1.000000,1.000000,1.000000")))
    (Game|SpawnActorfromClass (Variables|Default|GetClassOfBP) _output_get "AdjustIfPossibleButAlwaysSpawn" 0 0)
    ;[1 1 1] Remove Examine Menus from the screen
    (Variables|/Script/Engine.PlayerController|SetbShowMouseCursor _returnvalue false)
    (Widget|RemovefromParent (Variables|Default|GetExamineMenu))
    (Input|SetInputModeGameOnly _returnvalue)
    (bind _asfirst_person_hud (Utilities|Casting|CastToFirstPersonHUD (HUD|GetHUD (Game|GetPlayerController 0)))
      (:then
        (Variables|/Game/Quest2_BLueprints/CVInvInterface/Blueprints/FirstPersonHUD.FirstPersonHUD_C|SetShowCrossHairs _asfirst_person_hud true))
      (:CastFailed
        (Development|PrintString "Cant failed due to being unable to find a valid HUD within the Player Controller")))))

(event Custom|ExamineMenuKickoff
  (bind _returnvalue (Game|GetPlayerController 0))
  (bind _returnvalue_2 (Game|GetPlayerController 0))
  (bind _returnvalue_3 (Game|GetPlayerCharacter 0))
  (bind _pickupmesh (Variables|Default|GetPickupMesh))
  (bind (_outlocation _outrotation) (Actor|GetActorEyesViewPoint _returnvalue_3))
  (bind _returnvalue_4 (Transformation|GetComponentVelocity _pickupmesh))
  (bind (_x _y _z) (Math|Vector|BreakVector _returnvalue_4))
  ;[1 1 1] Clicking on an item in level initiates this Event from First Person Character Blueprint
  ;[1 1 1] Is OBJECT is moving, falling or shaking a little do nothing because a moving object may inherit movement before the next action takes place causing it to be Spawned incorrectly later.
  (if (< _x 1e+01)
    (if (< _y 1e+01)
      (if (< _z 1e+01)
        ;[1 0.0175 0.0844] Examine Object Closer
        ;;[1 1 1] Is there already an item being examined? If yes, do nothing, If no, continue. This prevents user from clicking on an item in level while Examine Menu is open.
        (if (not (Variables|Default|GetbHaveItemInHand))
          ;;[1 1 1] Gets Invpanelopen variable from FPCharacter to tell if Inventory is open or not. If it is, do nothing (Prevents user from clicking on item in level while Inventory is open), if not open Examine menu
          (if (not (stale EventInventoryIsOpen InvPanelOpen))
            ;;[1 1 1] Sends message to FPC to freeze in place and hand over control to User Interface, prevents user from moving while examining an item.
            (Class|BPIFreezePlayer|FreezePlayer(Message) (Game|GetPlayerCharacter 0) true)
            ;;[1 1 1] Sends message to FPC to set variables for hiding crosshair and displaying Examine Menu
            (bind _asfirst_person_hud (Utilities|Casting|CastToFirstPersonHUD (HUD|GetHUD (Game|GetPlayerController 0)))
              (:then
                (Variables|/Game/Quest2_BLueprints/CVInvInterface/Blueprints/FirstPersonHUD.FirstPersonHUD_C|SetShowCrossHairs _asfirst_person_hud false)
                (Variables|/Game/Quest2_BLueprints/CVInvInterface/Blueprints/FirstPersonHUD.FirstPersonHUD_C|SetShowExamine _asfirst_person_hud false)
                (Variables|Default|SetbHaveItemInHand true)
                ;;[0.9998 1 0.3997] Enable Input of keyboard and mouse
                (Input|EnableInput (Game|GetPlayerController 0))
                (Variables|Default|SetCameraLocation (Math|Transform|MakeTransform (+ _outlocation (Math|Vector|RotateVector (Variables|Default|GetExamineOffset) _outrotation)) _outrotation "1.000000,1.000000,1.000000"))
                ;;[1 1 1] Temporarily Hide the PickupMesh from the Level while examining it.
                (Development|SetHiddeninGame (Variables|Default|GetPickupMesh) true false)
                ;;[1 1 1] Get the Inventory Class to be used when examining this object, and then Spawn this object at location of CameraLocation Variable
                (bind _returnvalue_5 (Game|SpawnActorfromClass (.InventoryClass (Utilities|Struct|BreakBS_InvInfoStruct (Variables|Default|GetItemInfo))) (Variables|Default|GetCameraLocation) "AdjustIfPossibleButDontSpawnIfColliding" 0 0))
                ;;[1 1 1] Set location of Sphere Pivot for rotating of item
                (Transformation|SetWorldTransform (Variables|Default|GetSpherePivot) (Variables|Default|GetCameraLocation) false false)
                ;;[1 1 1] Get the InvMesh (static mesh) to display and rotate for this particular Pickup Item - Promote to variables to be used elsewhere in BP
                (bind _asbp_inventory_actor (Utilities|Casting|CastToBP_InventoryActor _returnvalue_5)
                  (:then
                    (Variables|Default|SetMeshToRotate (Variables|/Game/Quest2_BLueprints/CVInvInterface/Blueprints/InventoryActorBPS/BP_InventoryActor.BP_InventoryActor_C|GetInvMesh _asbp_inventory_actor))
                    (Variables|Default|SetBPInventoryActor _asbp_inventory_actor)
                    ;;[1 1 1] Attach INV item to player character so it doenst move if player is shaking or moving/falling
                    (Class|SceneComponent|Attachto (Variables|Default|GetSpherePivot) (Variables|/Script/Engine.Character|GetCapsuleComponent (Game|GetPlayerCharacter 0)) "None" "KeepWorldPosition" true)
                    ;;[1 1 1] Determine if the item is takable as set in its blueprint
                    (if (Utilities|Enum|Equal(Enum) (Variables|Default|GetTakableOrNot) "NewEnumerator0")
                      ;;[1 1 1] Display UMG Examine for a TAKABLE Object
                      (Variables|/Script/Engine.PlayerController|SetbShowMouseCursor _returnvalue true)
                      (Input|SetInputModeGameandUI _returnvalue 0 "DoNotLock" false)
                      ;;;[1 1 1] Display Examine Menu for takable item
                      (bind _returnvalue_6 (UserInterface|CreateWidget "/Game/Quest2_BLueprints/CVInvInterface/Blueprints/Widgets/BPW_Examine.BPW_Examine_C"))
                      (Variables|Default|SetExamineMenu _returnvalue_6)
                      (Class|BPIObjectInfo|ObjectDescription(Message) (Variables|Default|GetExamineMenu) (Variables|Default|GetItemDescription) (.ItemName (Utilities|Struct|BreakBS_InvInfoStruct (Variables|Default|GetItemInfo))))
                      (UserInterface|Viewport|AddtoViewport (Variables|Default|GetExamineMenu) 0)
                      (else
                        ;;[1 1 1] Display UMG Examine Only  for a NON-Takable Object
                        (Variables|/Script/Engine.PlayerController|SetbShowMouseCursor _returnvalue_2 true)
                        (Input|SetInputModeGameandUI _returnvalue_2 0 "DoNotLock" false)
                        ;;;[1 1 1] Display Examine Only menu for NON-Takable item
                        (bind _returnvalue_7 (UserInterface|CreateWidget "/Game/Quest2_BLueprints/CVInvInterface/Blueprints/Widgets/BPW_ExamineOnly.BPW_ExamineOnly_C"))
                        (Variables|Default|SetExamineOnlyMenu _returnvalue_7)
                        (Class|BPIObjectInfo|ObjectDescription(Message) (Variables|Default|GetExamineOnlyMenu) (Variables|Default|GetItemDescription) (.ItemName (Utilities|Struct|BreakBS_InvInfoStruct (Variables|Default|GetItemInfo))))
                        (UserInterface|Viewport|AddtoViewport (Variables|Default|GetExamineOnlyMenu) 0))))
                  (:CastFailed
                    (Development|PrintString "Cast failed - could not find valid InventoryActor within the PickupBlueprint the user clicked on"))))
              (:CastFailed
                (Development|PrintString "Unable to find valid HUD within Player Controller")))))))))

(event EventInventoryIsOpen
  (params (InvPanelOpen :type Boolean))
  ;[1 0.0175 0.0844] Examine Object Closer
  ;;[1 1 1] Gets Invpanelopen variable from FPCharacter to tell if Inventory is open or not. If it is, do nothing (Prevents user from clicking on item in level while Inventory is open), if not open Examine menu
)

(event Input|AxisEvents|InputAxisTurn
  (params (AxisValue :type Float%20%28single-precision%29))
  ;[1 1 1] If not rotating ittem, give control back to Controller Yaw and Pitch
)

(event Input|AxisEvents|InputAxisLookUp
  (params (AxisValue :type Float%20%28single-precision%29))
  ;[1 1 1] If not rotating ittem, give control back to Controller Yaw and Pitch
)

(event Input|AxisEvents|InputAxisTumbleObject
  (params (AxisValue :type Float%20%28single-precision%29))
  ;[1 1 1] Rotate Object When Being Examined..Left Or Right Key input
  (if (Variables|Default|GetbHaveItemInHand)
    ;;[1 1 1] IF Mouse is benig clicked (held down) then attach InvMesh to Sphere Pivot. If not (released) Detach, and reset rotation of Sphere Pivot then reattach.
    (if (Game|Player|IsInputKeyDown (Game|GetPlayerController 0) "LeftMouseButton")
      (Class|SceneComponent|Attachto (Variables|Default|GetMeshToRotate) (Variables|Default|GetSpherePivot) "None" "KeepWorldPosition" true)
      ;[1 1 1] Rotates Sphere Pivot Mesh (of which InvMesh is parented to) Pitch (up and down mouse movement) up is tip forward down is tip back
      (Transformation|AddLocalRotation (Variables|Default|GetSpherePivot) (Math|Rotator|MakeRotator 0.0 (* (* (stale Input|AxisEvents|InputAxisLookUp AxisValue) 1.0) 4.0) 0.0) false false)
      (else
        ;;[1 1 1] Detach Mesh from Sphere Pivot - then Reset Sphere Pivot Rotation to Zero - Then Re-attached Mesh To Rotate to Sphere Pivot. This prevents Gimbal lock and backwards rotating.
        (Class|SceneComponent|DetachfromParent (Variables|Default|GetMeshToRotate) true true)
        (Transformation|SetWorldTransform (Variables|Default|GetSpherePivot) (Variables|Default|GetCameraLocation) false false)
        (Class|SceneComponent|Attachto (Variables|Default|GetMeshToRotate) (Variables|Default|GetSpherePivot) "None" "KeepWorldPosition" false)))
    (else
      ;[1 1 1] If not rotating ittem, give control back to Controller Yaw and Pitch
      (Pawn|Input|AddControllerYawInput (Game|GetPlayerCharacter 0) (stale Input|AxisEvents|InputAxisTurn AxisValue))
      (Pawn|Input|AddControllerPitchInput (Game|GetPlayerCharacter 0) (stale Input|AxisEvents|InputAxisLookUp AxisValue)))))

(event Input|AxisEvents|InputAxisTurnObject
  (params (AxisValue :type Float%20%28single-precision%29))
  ;[1 1 1] Rotate Object When Being Examined..Left Or Right Key input
  (if (Variables|Default|GetbHaveItemInHand)
    (if (Game|Player|IsInputKeyDown (Game|GetPlayerController 0) "LeftMouseButton")
      ;;[1 1 1] Attach Mesh to Rotate to Sphere Pivot
      (Class|SceneComponent|Attachto (Variables|Default|GetMeshToRotate) (Variables|Default|GetSpherePivot) "None" "KeepWorldPosition" true)
      ;[1 1 1] Rotates Sphere Pivot (Of which InvMesh is parented to) Yaw (turn left to right).
      (Transformation|AddLocalRotation (Variables|Default|GetSpherePivot) (Math|Rotator|MakeRotator 0.0 0.0 (* (* (stale Input|AxisEvents|InputAxisTurn AxisValue) -1.0) 4.0)) false false)
      (else
        ;;[1 1 1] Detach Mesh from Sphere Pivot - then Reset Sphere Pivot Rotation to Zero - Then Re-attached Mesh To Rotate to Sphere Pivot. This prevents Gimbal lock and backwards rotating.
        (Class|SceneComponent|DetachfromParent (Variables|Default|GetMeshToRotate) true true)
        (Transformation|SetWorldTransform (Variables|Default|GetSpherePivot) (Variables|Default|GetCameraLocation) false false)
        (Class|SceneComponent|Attachto (Variables|Default|GetMeshToRotate) (Variables|Default|GetSpherePivot) "None" "KeepWorldPosition" false)))
    (else
      ;[1 1 1] If not rotating ittem, give control back to Controller Yaw and Pitch
      (Pawn|Input|AddControllerYawInput (Game|GetPlayerCharacter 0) (stale Input|AxisEvents|InputAxisTurn AxisValue))
      (Pawn|Input|AddControllerPitchInput (Game|GetPlayerCharacter 0) (stale Input|AxisEvents|InputAxisLookUp AxisValue)))))

(fn ConstructionScript
  ;[1 1 1] Sets Default value of Render Custom Depth as Negative so items are not highlighted until hovered over
  (Rendering|SetRenderCustomDepth (Variables|Default|GetPickupMesh) false))

(fn PutItemBack
  (params (Character :type First%20Person%20Character%20Object%20Reference))
  (CallFunction|PuttheItemBack)
  (return true false))

(fn EndFocus
  (params (Character :type Character%20Object%20Reference))
  ;[1 1 1] Sets Custom Render Depth back to default value of negative - removing the highlight from the item
  (Rendering|SetRenderCustomDepth (Variables|Default|GetPickupMesh) false))

(fn BeginFocus
  (params (Character :type First%20Person%20Character%20Object%20Reference))
  ;[1 1 1] Sets render custom depth to ON allowing highlighting of item when hovering over
  (Rendering|SetRenderCustomDepth (Variables|Default|GetPickupMesh) true))

(fn OnExamine
  (params (Character :type First%20Person%20Character%20Object%20Reference))
  (CallFunction|ExamineMenuKickoff)
  (return true))

(fn INVwasPressedFunction
  (return false))

(fn DropItemPickupBase
  (CallFunction|DropItemfromMenu)
  (return false))

(fn ThrowItemfromEx
  (params (throwinput :type Boolean))
  (return false))