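; Shop component template that lets a player buy and sell data-table items for coins through a shop widget.
; Server events load items, check prices and adjust coins, while client events create the widget, push lists and balance, toggle input mode and show timed messages.
; Inventory integration is left as placeholders: buying only deducts coins, and the sell and sale-list logic is partly unwired until an inventory is connected.
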(event Custom|Server_OpenShop
  ;[1 0.02697 0] Server
  (CallFunction|ClientShopVisibility)
  (CallFunction|ClientWidgetUpdateCoins (Variables|Default|GetCoins)))

(event Custom|Server_BuyItem
  (params (ItemId :type Name))
  ;[1 0.02697 0] Server
  (CallFunction|ServerBuyItemFunction ItemId))

(event Custom|Client_MessageBox
  (params (Message_TExt :type Text))
  ;[1 1 1] Client update information on widget
  (Utilities|Messages Message_TExt))

(event Custom|Server_GiveItem
  (params (Id :type Name) (Price :type Float%20%28single-precision%29))
  ;[0 0.594 1] Please connect your invetory on this functions
  (if true ; If item finded on inventory
    (CallFunction|ServerRemoveCoins (* Price -1.0)) ; Removed coins
    (CallFunction|ClientMessageBox "Item Bought")))

(event Custom|Server_OpenSaleTab
  ;[0 0.594 1] Please connect your invetory on this functions
  (CallFunction|ServerOpenSaleTabFunction :!pinned true) ; Open function and connect invetory
)

(event Custom|Server_ShopItem_Init
  (bind _shopitems (Variables|Default|GetShopItems))
  ;[1 1 1] Initialization
  (bind _out_row (Utilities|GetDataTable)
    (:Row%20Found
      (Utilities|Array|Add _shopitems _out_row))
    (:Completed
      (CallFunction|ClientShopItemInit _shopitems))))

(event Custom|Client_ShopItem_Init
  (params (ShopItem :type Array%20of%20S%20Shop%20Struct%20Structures))
  ;[1 1 1] Initialization
  (Variables|/Game/EasyShopModule/UI/Blueprints/WBP_Shop_Interface.WBP_Shop_Interface_C|SetShopItem (Variables|Default|GetShopInterface) ShopItem)
  (CallFunction|ServerOpenShop))

(event Custom|Server_RemoveItem
  (params (Id :type Name) (Price :type Float%20%28single-precision%29))
  ;[0 0.594 1] Please connect your invetory on this functions
  (if true
    (CallFunction|ServerRemoveCoins Price)
    (CallFunction|ServerOpenSaleTab)
    (CallFunction|ClientMessageBox "Item sold")))

(event Custom|Client_SetSaleInventory
  (params (SaleInventory :type Array%20of%20S%20Sale%20Struct%20Structures))
  ;[1 1 1] Client update information on widget
  (Variables|/Game/EasyShopModule/UI/Blueprints/WBP_Shop_Interface.WBP_Shop_Interface_C|SetSaleInventory (Variables|Default|GetShopInterface) SaleInventory)
  (CallFunction|ClientUpdateItemList))

(event Custom|Client_ShopVisibility
  ;[1 1 1] Client update information on widget
  (CallFunction|ClientOpenShopFunction (Game|GetPlayerController 0)))

(event Custom|Client_WidgetUpdateCoins
  (params (MyCoins :type Float%20%28single-precision%29))
  (bind _shopinterface (Variables|Default|GetShopInterface))
  ;[1 1 1] Client update information on widget
  (Utilities|IsValid _shopinterface
    (:Is%20Valid
      (Variables|/Game/EasyShopModule/UI/Blueprints/WBP_Shop_Interface.WBP_Shop_Interface_C|SetMyCoins _shopinterface MyCoins)
      (CallFunction|ClientUpdateItemList))))

(event Custom|Server_RemoveCoins
  (params (Count :type Float%20%28single-precision%29))
  ;[1 0.02697 0] Server
  (bind _newcoins (CallFunction|ServerChangeCoins Count))
  (CallFunction|ClientWidgetUpdateCoins _newcoins))

(event Custom|Server_SaleItem
  (params (Id :type Name))
  ;[0 0.594 1] Please connect your invetory on this functions
  (CallFunction|ServerSaleItenFunction Id :!pinned true) ; Open function and connect invetory
)

(event Custom|Client_ShopUnvisibility
  ;[1 1 1] Client update information on widget
  (CallFunction|ClientCloseShopFunction (Game|GetPlayerController 0)))

(event Custom|Server_closeShop
  ;[1 0.02697 0] Server
  (CallFunction|ClientShopUnvisibility))

(event Custom|Client_Initialization
  ;[1 1 1] Initialization
  (if (Pawn|IsLocallyControlled (Variables|/Script/Engine.Actor|GetInstigator (Components|GetOwner)))
    (CallFunction|Initialization)))

(event Custom|Client_UpdateItemList
  ;[1 1 1] Client update information on widget
  (Default|UpdateItemList (Variables|Default|GetShopInterface)))

(fn Initialization
  (bind _returnvalue (UserInterface|CreateWidget "/Game/EasyShopModule/UI/Blueprints/WBP_Shop_Interface.WBP_Shop_Interface_C"))
  (bind _output_get (Variables|Default|SetShopInterface _returnvalue))
  (CallFunction|ServerShopItemInit)
  (Variables|/Game/EasyShopModule/UI/Blueprints/WBP_Shop_Interface.WBP_Shop_Interface_C|SetShopComponent _output_get self)
  (Variables|/Game/EasyShopModule/UI/Blueprints/WBP_Shop_Interface.WBP_Shop_Interface_C|SetSlotName _output_get (Variables|Default|GetSlotName))
  (Default|Initialization _output_get)
  (bind _returnvalue_2 (SaveGame|DoesSaveGameExist (Variables|Default|GetSlotName)))
  (if _returnvalue_2
    _
    (else
      (Variables|/Game/EasyShopModule/UI/Blueprints/WBP_Shop_Interface.WBP_Shop_Interface_C|SetCoinsFilter _output_get (Variables|Default|GetCoinsFilter))
      (Variables|/Game/EasyShopModule/UI/Blueprints/WBP_Shop_Interface.WBP_Shop_Interface_C|SetCategory_View _output_get (Variables|Default|GetCategory_View))
      (Variables|/Game/EasyShopModule/UI/Blueprints/WBP_Shop_Interface.WBP_Shop_Interface_C|SetTopBar_View _output_get (Variables|Default|GetTopBar_View))
      (Variables|/Game/EasyShopModule/UI/Blueprints/WBP_Shop_Interface.WBP_Shop_Interface_C|SetItem_View _output_get (Variables|Default|GetItem_View))))
  (UserInterface|Viewport|AddtoViewport _output_get 0))

(fn ServerBuyItemFunction
  (params (InputPin :type Name))
  (bind _array_element (Utilities|Array|ForEachLoopwithBreak (Variables|Default|GetShopItems) :!label _label)
    (:LoopBody
      (if (Utilities|Name|Equal(Name) (Utilities|Struct|BreakSShop_Struct _array_element) InputPin)
        (Utilities|FlowControl|Sequence
          (:then_0
            (if (< (- (Variables|Default|GetCoins) (Utilities|Struct|BreakSShop_Struct _array_element)) 0.0)
              (CallFunction|ClientMessageBox "Not enough coins")
              (else
                (CallFunction|ServerGiveItem InputPin (Utilities|Struct|BreakSShop_Struct _array_element)))))
          (:then_1
            (goto _label Break)))))))

(fn ServerOpenSaleTabFunction
  (Utilities|Array|Clear (Variables|Default|GetSaleInventory)))

(fn ServerSaleItemFunction
  (bind _array_element (Utilities|Array|ForEachLoopwithBreak (Variables|Default|GetShopItems) :!label _label)
    (:LoopBody
      ;[1 1 1] Inventory array
      (Utilities|Array|ForEachLoopwithBreak (Variables|Default|GetShopItems)
        (:LoopBody
          (if (Utilities|Name|Equal(Name) "None" "None")
            (Utilities|FlowControl|Sequence
              (:then_1
                (if (Utilities|Name|Equal(Name) (.Id (Utilities|Struct|BreakSShop_Struct _array_element)) "None")
                  (Utilities|FlowControl|Sequence
                    (:then_0
                      (CallFunction|ServerRemoveItem "None" (Utilities|Struct|BreakSShop_Struct _array_element)))
                    (:then_1
                      (goto _label Break))))))))))))

(fn ServerChangeCoins
  (params (Coins :type Float%20%28single-precision%29))
  (bind _output_get (Variables|Default|SetCoins (+ Coins (Variables|Default|GetCoins))))
  (return _output_get))

(fn ClientCloseShopFunction
  (params (PlayerController :type Player%20Controller%20Object%20Reference))
  (Input|SetInputModeGameOnly PlayerController)
  (Variables|/Script/Engine.PlayerController|SetbShowMouseCursor PlayerController false)
  (Variables|/Game/EasyShopModule/UI/Blueprints/WBP_Shop_Interface.WBP_Shop_Interface_C|SetShopVisibility (Variables|Default|GetShopInterface) "Collapsed"))

(fn ClientOpenShopFunction
  (params (PlayerController :type Player%20Controller%20Object%20Reference))
  (bind _shopinterface (Variables|Default|GetShopInterface))
  (Utilities|IsValid _shopinterface
    (:Is%20Valid
      (Input|SetInputModeGameandUI PlayerController _shopinterface "DoNotLock" false)
      (Variables|/Script/Engine.PlayerController|SetbShowMouseCursor PlayerController true)
      (Variables|/Game/EasyShopModule/UI/Blueprints/WBP_Shop_Interface.WBP_Shop_Interface_C|SetShopVisibility _shopinterface "Visible"))
    (:Is%20Not%20Valid
      (CallFunction|ClientInitialization))))

(fn ServerSaleItenFunction
  (params (InputPin :type Name))
  (bind _array_element (Utilities|Array|ForEachLoopwithBreak (Variables|Default|GetShopItems))))