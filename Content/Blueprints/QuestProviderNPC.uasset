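; Quest-giver NPC that plays a timed dialogue when overlapped and then shows the player an objective.
; BeginPlay makes the first ThirdPersonCharacter ignore input until the dialogue loop completes.
; Any overlap creates a Quest widget and feeds it DialoguesOfQuest lines through a delayed loop, adding an Objective widget after a pause at a hard-coded index.
; Completion removes the Quest widget and restores input.
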(event EventBeginPlay
  (bind _outactors (Actor|GetAllActorsOfClass "/Game/Blueprints/ThirdPersonCharacter.ThirdPersonCharacter_C"))
  (Default|IgnoreInput (Utilities|Array|Get(acopy) _outactors)))

(event Collision|EventActorBeginOverlap
  (params (OtherActor :type Actor%20Object%20Reference))
  (bind _returnvalue (UserInterface|CreateWidget "/Game/Blueprints/Quest.Quest_C" (Game|GetPlayerController 0)))
  (bind _output_get (Variables|Default|SetQuest%20Widget _returnvalue))
  (UserInterface|Viewport|AddtoViewport _output_get 0)
  (bind (_array_element _array_index) (Utilities|ForEachLoopDelay (Variables|Default|GetDialogues%20of%20Quest) 0.8)
    (:Loop%20Body
      (if (== _array_index 3)
        (Variables|/Game/Blueprints/Quest.Quest_C|SetQuestDialogues (Variables|Default|GetQuest%20Widget) _array_element)
        (Utilities|FlowControl|Delay 1.0)
        (bind _returnvalue_2 (UserInterface|CreateWidget "/Game/Blueprints/Objective.Objective_C"))
        (UserInterface|Viewport|AddtoViewport _returnvalue_2 0)
        (else
          (Variables|/Game/Blueprints/Quest.Quest_C|SetQuestDialogues (Variables|Default|GetQuest%20Widget) _array_element))))
    (:Completed
      (Widget|RemovefromParent (Variables|Default|GetQuest%20Widget))
      (bind _outactors (Actor|GetAllActorsOfClass "/Game/Blueprints/ThirdPersonCharacter.ThirdPersonCharacter_C"))
      (Default|ResetIgnoreInput (Utilities|Array|Get(acopy) _outactors)))))

(event EventTick
  (params (DeltaSeconds :type Float%20%28single-precision%29)))

(fn ConstructionScript)